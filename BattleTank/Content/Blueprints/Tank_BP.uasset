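; Tank pawn Blueprint that wires player input to the tank's aiming and movement components.
; On BeginPlay it hands the barrel and turret to TankAiming and the left and right tracks to TankMovement.
; Aim axes rotate an azimuth gimbal and spring arm, scaled by frame time, to orbit the view.
; Fire calls TankAiming, while move axes pass forward and turn intent to TankMovement.
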(event EventBeginPlay
  (Class|TankAimingComponent|Initialize (Variables|Default|GetTankAiming) (Variables|Default|GetBarrel) (Variables|Default|GetTankTurret))
  (Class|TankMovementComponent|Initialize (Variables|Default|GetTankMovement) (Variables|Default|GetLeft%20Track) (Variables|Default|GetRight%20Track)))

(event Collision|EventActorBeginOverlap
  (params (OtherActor :type Actor%20Object%20Reference)))

(event EventTick
  (params (DeltaSeconds :type Float%20%28single-precision%29)))

(event Input|ActionEvents|InputActionFireProjectile
  (params (Key :type Key%20Structure :default "AnyKey"))
  ;[1 1 1] Ballistics Input Binding
  (:Pressed
    (Class|TankAimingComponent|Fire (Variables|Default|GetTankAiming))))

(event Input|AxisEvents|InputAxisAimAzimuth
  (params (AxisValue :type Float%20%28single-precision%29))
  ;[1 1 1] Ballistics Input Binding
  (Transformation|AddLocalRotation (Variables|Default|GetAzGimbal) (Math|Rotator|MakeRotator 0.0 0.0 (* AxisValue (Utilities|Time|GetWorldDeltaSeconds) 1e+02)) false false))

(event Input|AxisEvents|InputAxisMoveForward
  (params (AxisValue :type Float%20%28single-precision%29))
  ;[1 1 1] Ballistics Input Binding
  (Class|TankMovementComponent|IntendMoveForward (Variables|Default|GetTankMovement) AxisValue))

(event Input|AxisEvents|InputAxisMoveRight
  (params (AxisValue :type Float%20%28single-precision%29))
  ;[1 1 1] Ballistics Input Binding
  (Class|TankMovementComponent|IntendTurnRight (Variables|Default|GetTankMovement) AxisValue))

(event Input|AxisEvents|InputAxisAimElevation
  (params (AxisValue :type Float%20%28single-precision%29))
  ;[1 1 1] Ballistics Input Binding
  (Transformation|AddLocalRotation (Variables|Default|GetSpringArm) (Math|Rotator|MakeRotator 0.0 (* AxisValue (Utilities|Time|GetWorldDeltaSeconds) 1e+02) 0.0) false false))

(fn ConstructionScript)